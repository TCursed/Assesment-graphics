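; Player inventory for laser puzzle cubes (booster, reflector, reducer), letting the player pick up, place and rotate them.
; E and R sphere-trace at the player's feet and use actor tags to store or yaw-rotate boxes.
; O and L cycle the selected slot, and left click spawns that cube at a grid-snapped point ahead, previewed by a wireframe updated on Tick.
; Item changes refresh the WB_Inventory widget.
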(event EventBeginPlay
  (bind _returnvalue (UserInterface|CreateWidget "/Game/Laser/WB_Inventory.WB_Inventory_C"))
  (bind _output_get (Variables|Default|SetInventoryWidgit _returnvalue))
  (UserInterface|Viewport|AddtoViewport _output_get 0)
  (Utilities|Array|Resize (Variables|Default|GetItems) 5)
  (Default|LoadInventory (Variables|Default|GetInventoryWidgit) self)
  (bind _returnvalue_2 (Game|SpawnActorfromClass "/Game/Laser/BP_BoxVisual.BP_BoxVisual_C" (Math|Conversions|ToTransform(Vector) (Transformation|GetActorLocation (Game|GetPlayerCharacter 0))) "Undefined" "MultiplyWithRoot" 0 0))
  (Variables|Default|SetBoxWireframe _returnvalue_2))

(event EventTick
  (params (DeltaSeconds :type Float%20%28single-precision%29))
  (bind _returnvalue (Game|GetPlayerCharacter 0))
  (bind _distancefromplayer (Variables|Default|GetDistanceFromPlayer))
  (bind _returnvalue_2 (Transformation|GetActorForwardVector _returnvalue))
  (bind _returnvalue_3 (Transformation|GetActorLocation _returnvalue))
  (bind _returnvalue_4 (* _returnvalue_2 _distancefromplayer))
  (bind _returnvalue_5 (+ _returnvalue_4 _returnvalue_3))
  (bind (_x _y _z) (Math|Vector|BreakVector _returnvalue_5))
  (Transformation|SetActorLocation (Variables|Default|GetBoxWireframe) (Math|Vector|MakeVector (Math|Conversions|ToFloat(Integer) (* (Math|Float|Round (/ _x 1e+02)) 100)) (Math|Conversions|ToFloat(Integer) (* (Math|Float|Round (/ _y 1e+02)) 100)) (- _z 94.0)) false false))

(event Input|KeyboardEvents|R
  (params (Key :type Key%20Structure :default "None"))
  (bind _returnvalue (Game|GetPlayerCharacter 0))
  (bind _returnvalue_2 (Transformation|GetActorLocation _returnvalue))
  (bind _returnvalue_3 (- _returnvalue_2 "0.000000,0.000000,65.000000"))
  (:Pressed
    (bind _outhit (Collision|SphereTraceForObjects _returnvalue_3 _returnvalue_3 1.2e+02 (Utilities|Array|MakeArray "ObjectTypeQuery7" "ObjectTypeQuery8" "ObjectTypeQuery9") false 0 "ForDuration"))
    (if (Utilities|Enum|Equal(Enum) (Utilities|String|ToString(Name) (Utilities|Array|Get(acopy) (Variables|/Script/Engine.Actor|GetTags (.HitActor (Collision|BreakHitResult _outhit))))) "Booster")
      (bind _asbooster_box (Utilities|Casting|CastToBoosterBox (.HitActor (Collision|BreakHitResult _outhit))))
      (Transformation|SetActorRotation _asbooster_box (Math|Rotator|MakeRotator (.Roll (Math|Rotator|BreakRotator (Transformation|GetActorRotation _asbooster_box))) (.Pitch (Math|Rotator|BreakRotator (Transformation|GetActorRotation _asbooster_box))) (+ (.Yaw (Math|Rotator|BreakRotator (Transformation|GetActorRotation _asbooster_box))) 9e+01)))
      (elif (Utilities|Enum|Equal(Enum) (Utilities|String|ToString(Name) (Utilities|Array|Get(acopy) (Variables|/Script/Engine.Actor|GetTags (.HitActor (Collision|BreakHitResult _outhit))))) "Reflector")
        (bind _asreflect_box (Utilities|Casting|CastToReflectBox (.HitActor (Collision|BreakHitResult _outhit))))
        (Transformation|SetActorRotation _asreflect_box (Math|Rotator|MakeRotator (.Roll (Math|Rotator|BreakRotator (Transformation|GetActorRotation _asreflect_box))) (.Pitch (Math|Rotator|BreakRotator (Transformation|GetActorRotation _asreflect_box))) (+ (.Yaw (Math|Rotator|BreakRotator (Transformation|GetActorRotation _asreflect_box))) 9e+01)))
        (elif (Utilities|Enum|Equal(Enum) (Utilities|String|ToString(Name) (Utilities|Array|Get(acopy) (Variables|/Script/Engine.Actor|GetTags (.HitActor (Collision|BreakHitResult _outhit))))) "Reducer")
          (bind _asreducer_box (Utilities|Casting|CastToReducerBox (.HitActor (Collision|BreakHitResult _outhit))))
          (Transformation|SetActorRotation _asreducer_box (Math|Rotator|MakeRotator (.Roll (Math|Rotator|BreakRotator (Transformation|GetActorRotation _asreducer_box))) (.Pitch (Math|Rotator|BreakRotator (Transformation|GetActorRotation _asreducer_box))) (+ (.Yaw (Math|Rotator|BreakRotator (Transformation|GetActorRotation _asreducer_box))) 9e+01))))))))

(event Input|MouseEvents|LeftMouseButton
  (params (Key :type Key%20Structure :default "None"))
  (bind _returnvalue (Game|GetPlayerCharacter 0))
  (bind _s_item (Utilities|Struct|MakeS_Item "" false))
  (bind _distancefromplayer (Variables|Default|GetDistanceFromPlayer))
  (bind _returnvalue_2 (Transformation|GetActorForwardVector _returnvalue))
  (bind _returnvalue_3 (Transformation|GetActorLocation _returnvalue))
  (bind _returnvalue_4 (* _returnvalue_2 _distancefromplayer))
  (bind _returnvalue_5 (+ _returnvalue_4 _returnvalue_3))
  (bind (_x _y _z) (Math|Vector|BreakVector _returnvalue_5))
  (bind _returnvalue_6 (/ _x 1e+02))
  (bind _returnvalue_7 (/ _y 1e+02))
  (bind _returnvalue_8 (Math|Float|Round _returnvalue_6))
  (bind _returnvalue_9 (Math|Float|Round _returnvalue_7))
  (bind _returnvalue_10 (* _returnvalue_8 100))
  (bind _returnvalue_11 (* _returnvalue_9 100))
  (bind _returnvalue_12 (Math|Conversions|ToFloat(Integer) _returnvalue_10))
  (bind _returnvalue_13 (Math|Conversions|ToFloat(Integer) _returnvalue_11))
  (bind _returnvalue_14 (Math|Vector|MakeVector _returnvalue_12 _returnvalue_13 _z))
  (bind _returnvalue_15 (Math|Conversions|ToTransform(Vector) _returnvalue_14))
  (:Pressed
    (for (_array_element _array_index) (Variables|Default|GetItems)
      (if (> (.Quantity (Utilities|Struct|BreakS_Item _array_element)) 0)
        (if (and (Utilities|Enum|Equal(Enum) (.Name (Utilities|Struct|BreakS_Item _array_element)) (.Name (Utilities|Struct|BreakS_Item (Variables|Default|GetSelectedItem)))) (== (.Power (Utilities|Struct|BreakS_Item _array_element)) (.Power (Utilities|Struct|BreakS_Item (Variables|Default|GetSelectedItem)))))
          (if (== (.Quantity (Utilities|Struct|BreakS_Item _array_element)) 1)
            (Utilities|Array|SetArrayElem (Variables|Default|GetItems) _array_index _s_item)
            (else
              (Utilities|Array|SetArrayElem (Variables|Default|GetItems) _array_index (Utilities|Struct|MakeS_Item (.Name (Utilities|Struct|BreakS_Item _array_element)) (.Stackable (Utilities|Struct|BreakS_Item _array_element)) (- (.Quantity (Utilities|Struct|BreakS_Item _array_element)) 1) (.Power (Utilities|Struct|BreakS_Item _array_element))))))
          (Default|LoadInventory (Variables|Default|GetInventoryWidgit) self)
          (if (Utilities|Enum|Equal(Enum) (Utilities|String|ToString(Text) (.Name (Utilities|Struct|BreakS_Item (Variables|Default|GetSelectedItem)))) "BoosterCube")
            (Game|SpawnActorfromClass "/Game/Laser/BoosterBox.BoosterBox_C" _returnvalue_15 "AlwaysSpawn" "MultiplyWithRoot" 0 (Math|Conversions|ToFloat(Integer) (.Power (Utilities|Struct|BreakS_Item (Variables|Default|GetSelectedItem)))) (Variables|Default|GetSelectedItem) "(R=0.000000,G=0.000000,B=0.000000,A=0.000000)" 0 0)
            (Variables|Default|SetSelectedItem _s_item :!label _label)
            (elif (Utilities|Enum|Equal(Enum) (Utilities|String|ToString(Text) (.Name (Utilities|Struct|BreakS_Item (Variables|Default|GetSelectedItem)))) "LaserCube")
              (Game|SpawnActorfromClass "/Game/Laser/ReflectBox.ReflectBox_C" _returnvalue_15 "AlwaysSpawn" "MultiplyWithRoot" 0 (Variables|Default|GetSelectedItem) "(R=0.000000,G=0.000000,B=0.000000,A=0.000000)" 0 0)
              (goto _label)
              (elif (Utilities|Enum|Equal(Enum) (Utilities|String|ToString(Text) (.Name (Utilities|Struct|BreakS_Item (Variables|Default|GetSelectedItem)))) "ReducerCube")
                (Game|SpawnActorfromClass "/Game/Laser/ReducerBox.ReducerBox_C" _returnvalue_15 "AlwaysSpawn" "MultiplyWithRoot" 0 (Math|Conversions|ToFloat(Integer) (.Power (Utilities|Struct|BreakS_Item (Variables|Default|GetSelectedItem)))) (Variables|Default|GetSelectedItem) "(R=0.000000,G=0.000000,B=0.000000,A=0.000000)" 0 0)))))))))

(event Input|KeyboardEvents|O
  (params (Key :type Key%20Structure :default "None"))
  (:Pressed
    (if (== (Variables|Default|GetIndex) 5)
      (bind _output_get (Variables|Default|SetIndex 0))
      (Variables|Default|SetSelectedItem (Utilities|Array|Get(acopy) (Variables|Default|GetItems) _output_get))
      (else
        (bind _output_get_2 (Variables|Default|SetIndex (+ (Variables|Default|GetIndex) 1)))
        (Variables|Default|SetSelectedItem (Utilities|Array|Get(acopy) (Variables|Default|GetItems) _output_get_2))))))

(event Input|KeyboardEvents|L
  (params (Key :type Key%20Structure :default "None"))
  (:Pressed
    (if (== (Variables|Default|GetIndex) 0)
      (bind _output_get (Variables|Default|SetIndex 5))
      (Variables|Default|SetSelectedItem (Utilities|Array|Get(acopy) (Variables|Default|GetItems) _output_get))
      (else
        (bind _output_get_2 (Variables|Default|SetIndex (- (Variables|Default|GetIndex) 1)))
        (Variables|Default|SetSelectedItem (Utilities|Array|Get(acopy) (Variables|Default|GetItems) _output_get_2))))))

(event Input|KeyboardEvents|E
  (params (Key :type Key%20Structure :default "None"))
  (bind _returnvalue (Game|GetPlayerCharacter 0))
  (bind _returnvalue_2 (Transformation|GetActorLocation _returnvalue))
  (bind _returnvalue_3 (- _returnvalue_2 "0.000000,0.000000,65.000000"))
  (:Pressed
    (bind _outhit (Collision|SphereTraceForObjects _returnvalue_3 _returnvalue_3 1.2e+02 (Utilities|Array|MakeArray "ObjectTypeQuery7" "ObjectTypeQuery8" "ObjectTypeQuery9") false 0 "ForDuration"))
    (if (Utilities|Enum|Equal(Enum) (Utilities|String|ToString(Name) (Utilities|Array|Get(acopy) (Variables|/Script/Engine.Actor|GetTags (.HitActor (Collision|BreakHitResult _outhit))))) "Booster")
      (bind _asbooster_box (Utilities|Casting|CastToBoosterBox (.HitActor (Collision|BreakHitResult _outhit))))
      (for (_array_element _array_index) (Variables|Default|GetItems)
        (Utilities|IsValid _asbooster_box
          (:Is%20Valid
            (if (Math|Boolean|ANDBoolean (Utilities|Enum|Equal(Enum) (.Name (Utilities|Struct|BreakS_Item _array_element)) (.Name (Utilities|Struct|BreakS_Item (Variables|/Game/Laser/BoosterBox.BoosterBox_C|GetItem _asbooster_box)))) (.Stackable (Utilities|Struct|BreakS_Item (Variables|/Game/Laser/BoosterBox.BoosterBox_C|GetItem _asbooster_box))) (== (.Power (Utilities|Struct|BreakS_Item _array_element)) (.Power (Utilities|Struct|BreakS_Item (Variables|/Game/Laser/BoosterBox.BoosterBox_C|GetItem _asbooster_box)))))
              (Utilities|Array|SetArrayElem (Variables|Default|GetItems) 0 (Utilities|Struct|MakeS_Item (.Name (Utilities|Struct|BreakS_Item (Variables|/Game/Laser/BoosterBox.BoosterBox_C|GetItem _asbooster_box))) (.Stackable (Utilities|Struct|BreakS_Item (Variables|/Game/Laser/BoosterBox.BoosterBox_C|GetItem _asbooster_box))) (+ (.Quantity (Utilities|Struct|BreakS_Item _array_element)) (.Quantity (Utilities|Struct|BreakS_Item (Variables|/Game/Laser/BoosterBox.BoosterBox_C|GetItem _asbooster_box)))) (.Power (Utilities|Struct|BreakS_Item (Variables|/Game/Laser/BoosterBox.BoosterBox_C|GetItem _asbooster_box)))))
              (Default|LoadInventory (Variables|Default|GetInventoryWidgit) self :!label _label)
              (Actor|DestroyActor _asbooster_box)
              (elif (== (.Quantity (Utilities|Struct|BreakS_Item _array_element)) 0)
                (Utilities|Array|SetArrayElem (Variables|Default|GetItems) _array_index (Variables|/Game/Laser/BoosterBox.BoosterBox_C|GetItem _asbooster_box))
                (Variables|Default|SetSelectedItem (Variables|/Game/Laser/BoosterBox.BoosterBox_C|GetItem _asbooster_box))
                (Variables|Default|SetIndex _array_index)
                (goto _label))))))
      (elif (Utilities|Enum|Equal(Enum) (Utilities|String|ToString(Name) (Utilities|Array|Get(acopy) (Variables|/Script/Engine.Actor|GetTags (.HitActor (Collision|BreakHitResult _outhit))))) "Reflector")
        (bind _asreflect_box (Utilities|Casting|CastToReflectBox (.HitActor (Collision|BreakHitResult _outhit))))
        (for (_array_element_2 _array_index_2) (Variables|Default|GetItems)
          (Utilities|IsValid _asreflect_box
            (:Is%20Valid
              (if (Math|Boolean|ANDBoolean (Utilities|Enum|Equal(Enum) (.Name (Utilities|Struct|BreakS_Item _array_element_2)) (.Name (Utilities|Struct|BreakS_Item (Variables|/Game/Laser/ReflectBox.ReflectBox_C|GetItem _asreflect_box)))) (.Stackable (Utilities|Struct|BreakS_Item (Variables|/Game/Laser/ReflectBox.ReflectBox_C|GetItem _asreflect_box))) (== (.Power (Utilities|Struct|BreakS_Item _array_element_2)) (.Power (Utilities|Struct|BreakS_Item (Variables|/Game/Laser/ReflectBox.ReflectBox_C|GetItem _asreflect_box)))))
                (Utilities|Array|SetArrayElem (Variables|Default|GetItems) 0 (Utilities|Struct|MakeS_Item (.Name (Utilities|Struct|BreakS_Item (Variables|/Game/Laser/ReflectBox.ReflectBox_C|GetItem _asreflect_box))) (.Stackable (Utilities|Struct|BreakS_Item (Variables|/Game/Laser/ReflectBox.ReflectBox_C|GetItem _asreflect_box))) (+ (.Quantity (Utilities|Struct|BreakS_Item _array_element_2)) (.Quantity (Utilities|Struct|BreakS_Item (Variables|/Game/Laser/ReflectBox.ReflectBox_C|GetItem _asreflect_box)))) (.Power (Utilities|Struct|BreakS_Item (Variables|/Game/Laser/ReflectBox.ReflectBox_C|GetItem _asreflect_box)))))
                (Default|LoadInventory (Variables|Default|GetInventoryWidgit) self :!label _label_2)
                (Actor|DestroyActor _asreflect_box)
                (elif (== (.Quantity (Utilities|Struct|BreakS_Item _array_element_2)) 0)
                  (Utilities|Array|SetArrayElem (Variables|Default|GetItems) _array_index_2 (Variables|/Game/Laser/ReflectBox.ReflectBox_C|GetItem _asreflect_box))
                  (Variables|Default|SetSelectedItem (Variables|/Game/Laser/ReflectBox.ReflectBox_C|GetItem _asreflect_box))
                  (Variables|Default|SetIndex _array_index_2)
                  (goto _label_2))))))
        (elif (Utilities|Enum|Equal(Enum) (Utilities|String|ToString(Name) (Utilities|Array|Get(acopy) (Variables|/Script/Engine.Actor|GetTags (.HitActor (Collision|BreakHitResult _outhit))))) "Reducer")
          (bind _asreducer_box (Utilities|Casting|CastToReducerBox (.HitActor (Collision|BreakHitResult _outhit))))
          (for (_array_element_3 _array_index_3) (Variables|Default|GetItems)
            (Utilities|IsValid _asreducer_box
              (:Is%20Valid
                (if (Math|Boolean|ANDBoolean (Utilities|Enum|Equal(Enum) (.Name (Utilities|Struct|BreakS_Item _array_element_3)) (.Name (Utilities|Struct|BreakS_Item (Variables|/Game/Laser/ReducerBox.ReducerBox_C|GetItem _asreducer_box)))) (.Stackable (Utilities|Struct|BreakS_Item (Variables|/Game/Laser/ReducerBox.ReducerBox_C|GetItem _asreducer_box))) (== (.Power (Utilities|Struct|BreakS_Item _array_element_3)) (.Power (Utilities|Struct|BreakS_Item (Variables|/Game/Laser/ReducerBox.ReducerBox_C|GetItem _asreducer_box)))))
                  (Utilities|Array|SetArrayElem (Variables|Default|GetItems) 0 (Utilities|Struct|MakeS_Item (.Name (Utilities|Struct|BreakS_Item (Variables|/Game/Laser/ReducerBox.ReducerBox_C|GetItem _asreducer_box))) (.Stackable (Utilities|Struct|BreakS_Item (Variables|/Game/Laser/ReducerBox.ReducerBox_C|GetItem _asreducer_box))) (+ (.Quantity (Utilities|Struct|BreakS_Item _array_element_3)) (.Quantity (Utilities|Struct|BreakS_Item (Variables|/Game/Laser/ReducerBox.ReducerBox_C|GetItem _asreducer_box)))) (.Power (Utilities|Struct|BreakS_Item (Variables|/Game/Laser/ReducerBox.ReducerBox_C|GetItem _asreducer_box)))))
                  (Default|LoadInventory (Variables|Default|GetInventoryWidgit) self :!label _label_3)
                  (Actor|DestroyActor _asreducer_box)
                  (elif (== (.Quantity (Utilities|Struct|BreakS_Item _array_element_3)) 0)
                    (Utilities|Array|SetArrayElem (Variables|Default|GetItems) _array_index_3 (Variables|/Game/Laser/ReducerBox.ReducerBox_C|GetItem _asreducer_box))
                    (Variables|Default|SetSelectedItem (Variables|/Game/Laser/ReducerBox.ReducerBox_C|GetItem _asreducer_box))
                    (Variables|Default|SetIndex _array_index_3)
                    (goto _label_3)))))))))))

(fn NewFunction
  (params (InRot :type Rotator%20%28by%20ref%29)))