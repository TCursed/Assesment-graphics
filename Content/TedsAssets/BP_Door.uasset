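; BP_Door is a double sliding door that opens on DoorOpen_Event and shuts after the player is detected at it.
; DoorTimeline lerps both panels apart by OpenOffset while Closed is true.
; Tick box-traces at the mesh, replaces player inventory slots of quantity one with empty items and refreshes the widget.
; After a delay it clears Closed and runs TimelineClose, whose identical lerp endpoints snap the panels shut rather than sliding them.
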(event Custom|DoorOpen_Event
  (bind _closedlocationl (Variables|Default|GetClosedLocationL))
  (bind _closedlocationr (Variables|Default|GetClosedLocationR))
  (bind _openoffset (Variables|Default|GetOpenOffset))
  (if (Variables|Default|GetClosed)
    (bind _slidea (Timeline|DoorTimeline Play)
      (:Update
        (Transformation|SetRelativeLocation (Variables|Default|GetDoorL) (Math|Vector|Lerp(Vector) _closedlocationl (- _closedlocationl _openoffset) _slidea) false false)
        (Transformation|SetRelativeLocation (Variables|Default|GetDoorR) (Math|Vector|Lerp(Vector) _closedlocationr (+ _openoffset _closedlocationr) _slidea) false false)))))

(event EventBeginPlay
  (Variables|Default|SetClosedLocationL (Variables|/Script/Engine.SceneComponent|GetRelativeLocation (Variables|Default|GetDoorL)))
  (Variables|Default|SetClosedLocationR (Variables|/Script/Engine.SceneComponent|GetRelativeLocation (Variables|Default|GetDoorR))))

(event EventTick
  (params (DeltaSeconds :type Float%20%28single-precision%29))
  (bind _returnvalue (Game|GetPlayerCharacter 0))
  (bind _closedlocationl (Variables|Default|GetClosedLocationL))
  (bind _closedlocationr (Variables|Default|GetClosedLocationR))
  (bind _openoffset (Variables|Default|GetOpenOffset))
  (bind _staticmesh (Variables|Default|GetStaticMesh))
  (bind _returnvalue_2 (Math|Vector|GetForwardVector _staticmesh))
  (bind _returnvalue_3 (Transformation|GetWorldLocation _staticmesh))
  (bind _returnvalue_4 (- _returnvalue_3 _returnvalue_2))
  (if (Variables|Default|GetClosed)
    (bind _outhit (Class|KismetSystemLibrary|BoxTraceSinglebyProfile _returnvalue_4 _returnvalue_4 "100.000000,4.000000,100.000000" (Transformation|GetWorldRotation _staticmesh) "NoCollision" false 0 "None" true))
    (if (== (.HitActor (Collision|BreakHitResult _outhit)) _returnvalue)
      (bind _asbp_third_person_character (Utilities|Casting|CastToBP_ThirdPersonCharacter _returnvalue))
      (Utilities|FlowControl|Sequence
        (:then_0
          (bind _invtcomp (Default|GetInvt _asbp_third_person_character))
          (for (_array_element _array_index) (Variables|/Game/TedsAssets/Inventory/BP_Inventory.BP_Inventory_C|GetItems _invtcomp)
            (if (== 1 (.Quantity (Utilities|Struct|BreakS_Item _array_element)))
              (Utilities|Array|SetArrayElem (Variables|/Game/TedsAssets/Inventory/BP_Inventory.BP_Inventory_C|GetItems _invtcomp) _array_index (Utilities|Struct|MakeS_Item "" true))
              (Default|LoadInventory (Variables|/Game/TedsAssets/Inventory/BP_Inventory.BP_Inventory_C|GetInventoryWidgit _invtcomp) _invtcomp))))
        (:then_1
          (Utilities|FlowControl|Delay 2.0)
          (Variables|Default|SetClosed false)
          (bind _newtrack_0 (Timeline|TimelineClose Play)
            (:Update
              (Transformation|SetRelativeLocation (Variables|Default|GetDoorL) (Math|Vector|Lerp(Vector) _closedlocationl (+ (- _closedlocationl _openoffset) _openoffset) _newtrack_0) false false)
              (Transformation|SetRelativeLocation (Variables|Default|GetDoorR) (Math|Vector|Lerp(Vector) _closedlocationr (- _openoffset (- _openoffset _closedlocationr)) _newtrack_0) false false))))))))

(fn ConstructionScript)